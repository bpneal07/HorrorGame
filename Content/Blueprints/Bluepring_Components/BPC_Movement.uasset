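; Movement component that handles sprinting with stamina and crouching for a player character passed in through Initialize.
; Looping function-name timers drain stamina while the player sprints and moves, then regenerate it after a retriggerable delay once sprinting stops.
; Crouching cancels the sprint timer and calls BP_L1-Character to resize its capsule.
; Each state sets the CharacterMovement max walk speed, and stamina changes print for debugging.
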(event `Start Sprint`
  ;[1 1 1] Start Sprint
  (if (`self.isCrouching`)
    (`self.End Crouch`))
  (if (and (> (`self.CurrentStamina`) (`self.MinStamina`)) (> (`KismetMathLibrary.VSize` (`Actor.GetVelocity` (`self.PlayerRef`))) 10.0))
    (`KismetSystemLibrary.K2_ClearTimer` null "Regenerate Stamina")
    (`self.Set Player Max Walk Speed` (`self.SprintSpeed`))
    (`KismetSystemLibrary.K2_SetTimer` null "Sprint Timer" 0.1 true)))

(event `Sprint Timer`
  ;[1 1 1] Sprint TImer
  (if (and (> (`self.CurrentStamina`) (`self.MinStamina`)) (> (`KismetMathLibrary.VSize` (`Actor.GetVelocity` (`self.PlayerRef`))) 10.0))
    (bind _output_get (set `self.CurrentStamina` (`KismetMathLibrary.FClamp` (- (`self.CurrentStamina`) 1.0) (`self.MinStamina`) (`self.MaxStamina`))))
    (`KismetSystemLibrary.PrintString` (`KismetStringLibrary.Conv_DoubleToString` _output_get))
    (if (<= (`self.CurrentStamina`) (`self.MinStamina`))
      (`self.Stop Sprint`))
    (else
      (`self.Stop Sprint`))))

(event `Stop Sprint`
  ;[1 1 1] Stop Sprinting
  (if (not (`self.isCrouching`))
    (`KismetSystemLibrary.K2_ClearTimer` null "Sprint Timer")
    (`self.Set Player Max Walk Speed` (`self.WalkSpeed`))
    (`KismetSystemLibrary.RetriggerableDelay` 5.0)
    (if (not (`KismetSystemLibrary.K2_IsTimerActive` null "Sprint Timer"))
      (`KismetSystemLibrary.K2_SetTimer` null "Regenerate Stamina" 0.03 true))))

(event `Regenerate Stamina`
  ;[1 1 1] Regenerate Stamina
  (bind _output_get (set `self.CurrentStamina` (`KismetMathLibrary.FClamp` (+ (`self.CurrentStamina`) 1.0) (`self.MinStamina`) (`self.MaxStamina`))))
  (`KismetSystemLibrary.PrintString` (`KismetStringLibrary.Conv_DoubleToString` _output_get))
  (if (>= (`self.CurrentStamina`) (`self.MaxStamina`))
    (`KismetSystemLibrary.K2_ClearTimer` null "Regenerate Stamina")))

(event `Start Crouch`
  (`KismetSystemLibrary.K2_ClearTimer` null "Sprint Timer")
  (`self.Set Player Max Walk Speed` (`self.CrouchSpeed`))
  (`/Game/GameBP/Level1/BP_L1-Character.Shorten Player Capsule` (cast `/Game/GameBP/Level1/BP_L1-Character` (`self.PlayerRef`) :!pure true))
  (set `self.isCrouching` true))

(event `End Crouch`
  (`self.Set Player Max Walk Speed` (`self.WalkSpeed`))
  (`/Game/GameBP/Level1/BP_L1-Character.Lengthen Player Capsule` (cast `/Game/GameBP/Level1/BP_L1-Character` (`self.PlayerRef`) :!pure true))
  (set `self.isCrouching` false))

(fn `Initialize`
  (params (Character :type "Character Object Reference"))
  (set `self.PlayerRef` Character)
  (set `CharacterMovementComponent.MaxWalkSpeed` (`self.WalkSpeed`) (`Character.CharacterMovement` (`self.PlayerRef`))))

(fn `Set Player Max Walk Speed`
  (params (MaxWalkSpeed :type "Float (single-precision)"))
  (set `CharacterMovementComponent.MaxWalkSpeed` MaxWalkSpeed (`Character.CharacterMovement` (`self.PlayerRef`))))