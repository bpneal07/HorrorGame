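; BP_LightSwitch is an interactable light switch actor that turns a referenced light on and off.
; Its Interact event checks that the Light reference is valid, then flips the visibility of that light's root component without propagating to child components.
; BeginPlay, overlap, Tick and the construction script add no logic of their own.
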(event `/Game/Blueprints/Interfaces/BPI_Interactions.Interact`
  (bind _rootcomponent (`Actor.RootComponent` (`self.Light`)))
  (`/Engine/EditorBlueprintResources/StandardMacros.IsValid` (`self.Light`)
    (:`Is Valid`
      (if (`SceneComponent.bVisible` _rootcomponent)
        (`SceneComponent.SetVisibility` _rootcomponent false false)
        (else
          (`SceneComponent.SetVisibility` _rootcomponent true false))))))

(fn `UserConstructionScript`
  (`parent.UserConstructionScript`))