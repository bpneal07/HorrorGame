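; Interactable door actor that toggles open and closed on Interact and swings away from the player.
; When opening, it takes the dot product of the player-to-door direction and the door's forward vector to pick a positive or negative quarter-turn swing.
; A timeline lerps the mesh's relative yaw to that angle and plays in reverse to close it.
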(event `/Game/Blueprints/Interfaces/BPI_Interactions.Interact`
  (if (`self.isDoorClosed`)
    (set `self.isDoorClosed` false)
    (set `self.DotProduct` (`KismetMathLibrary.Dot_VectorVector` (`KismetMathLibrary.Normal` (- (`self.K2_GetActorLocation` self) (`self.K2_GetActorLocation` (`self.PlayerRef`)))) (`self.GetActorForwardVector` self)))
    (bind (_direction _alpha) (`Timeline|OpenDoorTL` :!via `PlayFromStart` :!label _label)
      (:`Update`
        (`SceneComponent.K2_SetRelativeRotation` (`self.StaticMesh1`) (`KismetMathLibrary.MakeRotator` 0.0 0.0 (`KismetMathLibrary.Lerp` 0.0 (select `bool` (>= (`self.DotProduct`) 0.0) :`false` -90.0 :`true` 90.0) _alpha)) false false)))
    (else
      (set `self.isDoorClosed` true)
      (goto _label :!via `ReverseFromEnd`))))

(fn `UserConstructionScript`
  (`parent.UserConstructionScript`))